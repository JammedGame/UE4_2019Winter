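; SoundInput is a utility Blueprint that turns captured audio input into a normalized loudness value.
; An audio capture component, activated at BeginPlay, reports envelope values that update the current, minimum and maximum readings.
; GetValue rescales the current reading against that self-adjusting range, returning a truncated percentage, the raw fraction and an active flag set above a threshold.
; PrintStatus prints the percentage while active.
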(event `self.ReceiveBeginPlay`
  (`ActorComponent.Activate` (`self.Audio`) false))

(event `self.Audio.OnAudioEnvelopeValue`
  (params (EnvelopeValue :type "Float (single-precision)"))
  (bind _output_get (set `self.RecordedValue` EnvelopeValue))
  (if (> _output_get (`self.MaxRecordedValue`))
    (set `self.MaxRecordedValue` _output_get))
  (if (< _output_get (`self.MinRecordedValue`))
    (set `self.MinRecordedValue` _output_get)))

(fn `CalculateValueByOffset`
  (returns (Value :type "Float (double-precision)"))
  (bind _minrecordedvalue (`self.MinRecordedValue`))
  (if (> (`self.MinRecordedValue`) (`self.MaxRecordedValue`))
    (return 0.0)
    (else
      (return (/ (- (`self.RecordedValue`) _minrecordedvalue) (- (`self.MaxRecordedValue`) _minrecordedvalue))))))

(fn `GetValue`
  (returns (Value :type Integer) (BaseValue :type "Float (double-precision)") (Active :type Boolean))
  (bind _value (`self.CalculateValueByOffset`))
  (return (`KismetMathLibrary.FTrunc` (* 100 _value)) _value (> _value (`self.Threshold`))))

(fn `PrintStatus`
  (bind (_value _basevalue _active) (`self.GetValue`))
  (if _active
    (`KismetSystemLibrary.PrintString` (`KismetStringLibrary.Conv_IntToString` _value))))

(fn `UserConstructionScript`
  (`AddComponent|NODE_AddAudioCaptureComponent-1`)
  (set `self.RecordedValue` 0.0)
  (set `self.MinRecordedValue` 1.0)
  (set `self.MaxRecordedValue` 0.0))